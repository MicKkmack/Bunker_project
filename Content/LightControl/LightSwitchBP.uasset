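; LightSwitchBP is a light switch that toggles lights sharing its LightIndex when the player presses Interaction nearby.
; On BeginPlay it collects every LightBP actor into LightArray.
; Overlapping the SwitchInteraction component enables input and opens a gate, and ending overlap reverses both.
; A press through the open gate loops over the array and calls ToggleLightsMessage on each matching light.
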(event `self.ReceiveBeginPlay`
  ;[1 1 1] when we begin game, get all lights, add them to light array
  (bind _outactors (`GameplayStatics.GetAllActorsOfClass` "/Game/LightControl/LightBP.LightBP_C"))
  (for _array_element _outactors
    (`KismetArrayLibrary.Array_Add` (`self.Light Array`) _array_element)))

(event `InputAction|Interaction`
  (params (Key :type "Key Structure"))
  (:`Pressed`
    ;[1 1 1 1 10] need to open gate to Enter it for an exit (think rl)
    (`/Engine/EditorBlueprintResources/StandardMacros.Gate` true :!label _label
      (:`Exit`
        ;[1 1 1 1 10] get light index from loop and check against light index from light switch , if both true then continue. If true toggle light, if false nothing
        (for _array_element (`self.Light Array`)
          (if (== (`/Game/LightControl/LightBP.Light Index` _array_element) (`self.Light Index`))
            (message `/Game/LightControl/LightInterface.Toggle Lights` _array_element)))))))

(event `self.SwitchInteraction.OnComponentBeginOverlap`
  (params (OverlappedComponent :type "PrimitiveComponent Object Reference") (OtherActor :type "Actor Object Reference") (OtherComp :type "PrimitiveComponent Object Reference") (OtherBodyIndex :type Integer) (bFromSweep :type Boolean) (SweepResult :type "HitResult Structure (by ref)"))
  ;[1 1 1] Input
  (`self.EnableInput` (`GameplayStatics.GetPlayerController` 0))
  (goto _label :!via `Open`))

(event `self.SwitchInteraction.OnComponentEndOverlap`
  (params (OverlappedComponent :type "PrimitiveComponent Object Reference") (OtherActor :type "Actor Object Reference") (OtherComp :type "PrimitiveComponent Object Reference") (OtherBodyIndex :type Integer))
  ;[1 1 1] Input
  (`self.DisableInput` (`GameplayStatics.GetPlayerController` 0))
  (goto _label :!via `Close`))

(fn `UserConstructionScript`)