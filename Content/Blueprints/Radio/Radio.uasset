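; Interactive radio actor that lets the first-person player pause and resume its sound.
; A Box overlap enables player input on the radio when BP_FirstPersonCharacter enters and disables it on exit.
; While input is enabled, each Interaction press flips the IsPaused flag and sets the paused state of RadioSound to match.
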(event `InputAction|Interaction`
  (params (Key :type "Key Structure"))
  (bind _radiosound (`self.RadioSound`))
  ;[1 1 1] Play sound
  (:`Pressed`
    (if (`self.Is Paused`)
      (`AudioComponent.SetPaused` _radiosound false)
      (set `self.Is Paused` false)
      (else
        (`AudioComponent.SetPaused` _radiosound true)
        (set `self.Is Paused` true)))))

(event `self.Box.OnComponentBeginOverlap`
  (params (OverlappedComponent :type "PrimitiveComponent Object Reference") (OtherActor :type "Actor Object Reference") (OtherComp :type "PrimitiveComponent Object Reference") (OtherBodyIndex :type Integer) (bFromSweep :type Boolean) (SweepResult :type "HitResult Structure (by ref)"))
  ;[1 1 1] Allow interaction
  (cast `/Game/FirstPerson/Blueprints/BP_FirstPersonCharacter` OtherActor)
  (`self.EnableInput` (`GameplayStatics.GetPlayerController` 0)))

(event `self.Box.OnComponentEndOverlap`
  (params (OverlappedComponent :type "PrimitiveComponent Object Reference") (OtherActor :type "Actor Object Reference") (OtherComp :type "PrimitiveComponent Object Reference") (OtherBodyIndex :type Integer))
  ;[1 1 1] Allow interaction
  (cast `/Game/FirstPerson/Blueprints/BP_FirstPersonCharacter` OtherActor)
  (`self.DisableInput` (`GameplayStatics.GetPlayerController` 0)))

(fn `UserConstructionScript`)