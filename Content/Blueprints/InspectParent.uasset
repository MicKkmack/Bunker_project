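; InspectParent is a parent Blueprint for items the player can inspect and rotate with the mouse.
; StartInspect moves player input from the inspecting character to the item.
; While either mouse button is held, mouse X and Y add roll and pitch to the Item's relative rotation through CombineRotators.
; Pressing Inspect hands input back to the character and calls Inspect on BP_FirstPersonCharacter.
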(event `Start Inspect`
  (params (Inspector :type "Pawn Object Reference"))
  (bind _returnvalue (`GameplayStatics.GetPlayerController` 0))
  ;[1 1 1] Start/Stop Inspect
  ;;[1 1 1] You control the item not character
  (`self.DisableInput` Inspector _returnvalue)
  (`self.EnableInput` _returnvalue))

(event `InputAction|Inspect`
  (params (Key :type "Key Structure"))
  (bind _returnvalue (`GameplayStatics.GetPlayerController` 0))
  ;[1 1 1] Start/Stop Inspect
  ;;[1 1 1] Stop inspecting
  (:`Pressed`
    (`self.DisableInput` _returnvalue)
    (`self.EnableInput` (stale `Start Inspect` Inspector) _returnvalue)
    (bind _asbp_first_person_character (cast `/Game/FirstPerson/Blueprints/BP_FirstPersonCharacter` (stale `Start Inspect` Inspector)))
    (`/Game/FirstPerson/Blueprints/BP_FirstPersonCharacter.Inspect` _asbp_first_person_character)))

(event `InputAxisKey|MouseX`
  (params (AxisValue :type "Float (single-precision)"))
  (bind _returnvalue (`GameplayStatics.GetPlayerController` 0))
  ;[1 1 1] Roate Item Controls
  (if (or (`PlayerController.IsInputKeyDown` _returnvalue "LeftMouseButton") (`PlayerController.IsInputKeyDown` _returnvalue "RightMouseButton"))
    (`SceneComponent.K2_SetRelativeRotation` (`self.Item`) (`KismetMathLibrary.ComposeRotators` (`SceneComponent.RelativeRotation` (`self.Item`)) (`KismetMathLibrary.MakeRotator` (* AxisValue -1.0))) false false)))

(event `InputAxisKey|MouseY`
  (params (AxisValue :type "Float (single-precision)"))
  (bind _returnvalue (`GameplayStatics.GetPlayerController` 0))
  ;[1 1 1] Roate Item Controls
  (if (or (`PlayerController.IsInputKeyDown` _returnvalue "LeftMouseButton") (`PlayerController.IsInputKeyDown` _returnvalue "RightMouseButton"))
    (`SceneComponent.K2_SetRelativeRotation` (`self.Item`) (`KismetMathLibrary.ComposeRotators` (`SceneComponent.RelativeRotation` (`self.Item`)) (`KismetMathLibrary.MakeRotator` 0.0 (* AxisValue -1.0))) false false)))

(fn `UserConstructionScript`)